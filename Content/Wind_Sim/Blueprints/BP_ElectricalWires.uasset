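; BP_ElectricalWires is an electrical pole actor that strings three cable components to a referenced NextElectricalPole.
; The construction script places each cable's end at the matching sphere on that pole, converted to local space, or destroys the cables without one.
; IsRandomHang applies one shared gravity scale to all cables and a sine-based sideways force to Cable1, computed only at construction.
; The ResetWires branch and event graph are empty.
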(event EventBeginPlay)

(event Collision|EventActorBeginOverlap
  (params (OtherActor :type Actor%20Object%20Reference)))

(event EventTick
  (params (DeltaSeconds :type Float%20%28single-precision%29)))

(fn ConstructionScript
  (bind _cablehang_1 (Variables|Default|GetCableHang_1))
  (if (Variables|Default|GetResetWires)
    _
    (else
      _))
  (Utilities|IsValid (Variables|Default|GetNextElectricalPole)
    (:Is%20Valid
      (Variables|/Script/CableComponent.CableComponent|SetEndLocation (Variables|Default|GetCable1) (Math|Transform|InverseTransformLocation (Transformation|GetActorTransform) (Transformation|GetWorldLocation (Variables|BP_ElectricalWires_C|GetSphere1 (Variables|Default|GetNextElectricalPole)))))
      (Variables|/Script/CableComponent.CableComponent|SetEndLocation (Variables|Default|GetCable2) (Math|Transform|InverseTransformLocation (Transformation|GetActorTransform) (Transformation|GetWorldLocation (Variables|BP_ElectricalWires_C|GetSphere2 (Variables|Default|GetNextElectricalPole)))))
      (Variables|/Script/CableComponent.CableComponent|SetEndLocation (Variables|Default|GetCable3) (Math|Transform|InverseTransformLocation (Transformation|GetActorTransform) (Transformation|GetWorldLocation (Variables|BP_ElectricalWires_C|GetSphere3 (Variables|Default|GetNextElectricalPole)))))
      (if (Variables|Default|GetIsRandomHang)
        (Variables|/Script/CableComponent.CableComponent|SetCableGravityScale (Variables|Default|GetCable1) _cablehang_1)
        (Variables|/Script/CableComponent.CableComponent|SetCableGravityScale (Variables|Default|GetCable2) _cablehang_1)
        (Variables|/Script/CableComponent.CableComponent|SetCableGravityScale (Variables|Default|GetCable3) _cablehang_1)
        (Variables|/Script/CableComponent.CableComponent|SetCableForce (Variables|Default|GetCable1) (Math|Vector|MakeVector 0.0 (* (Math|Trig|Sin(Radians) (* (Utilities|Time|GetWorldDeltaSeconds) 5.0)) 5e+02) 0.0))))
    (:Is%20Not%20Valid
      (Components|DestroyComponent (Variables|Default|GetCable2)))))